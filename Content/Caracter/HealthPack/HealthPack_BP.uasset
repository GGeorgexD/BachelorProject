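; Health pickup Blueprint that restores a Paladin to full health on overlap.
; Tick adds a small fixed local rotation every frame to spin the pack, independent of delta time.
; When the HP_BP component overlaps a Paladin_BP below 100 health, it sets health to 100, passes the value to CallHealth and destroys itself.
; A Paladin already at full health leaves the pack in place.
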(event OnComponentBeginOverlap(HP_BP)
  (params (OverlappedComponent :type Primitive%20Component%20Object%20Reference) (OtherActor :type Actor%20Object%20Reference) (OtherComp :type Primitive%20Component%20Object%20Reference) (OtherBodyIndex :type Integer) (bFromSweep :type Boolean) (SweepResult :type Hit%20Result%20Structure%20%28by%20ref%29))
  (bind _aspaladin_bp (Utilities|Casting|CastToPaladin_BP OtherActor))
  (Variables|Default|SetPaladinRef _aspaladin_bp)
  (if (< (Variables|/Game/Caracter/Paladin_BP.Paladin_BP_C|GetCurrentHealth _aspaladin_bp) 1e+02)
    (bind _output_get (Variables|/Game/Caracter/Paladin_BP.Paladin_BP_C|SetCurrentHealth (Variables|Default|GetPaladinRef) 1e+02))
    (Default|CallHealth (Variables|Default|GetPaladinRef) _output_get)
    (Actor|DestroyActor)))

(event EventBeginPlay)

(event Collision|EventActorBeginOverlap
  (params (OtherActor :type Actor%20Object%20Reference)))

(event EventTick
  (params (DeltaSeconds :type Float%20%28single-precision%29))
  (Class|Actor|AddActorLocalTransform (Math|Transform|MakeTransform "0, 0, 0" "0.000000,0.000000,1.000000" "1,1,1") false false))

(fn ConstructionScript)